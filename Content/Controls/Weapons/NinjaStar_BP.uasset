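; Ninja star weapon Blueprint that keeps its star component spinning.
; Each Tick calls the parent Tick, then adds RotationIncrement to the NinjaStar component's relative yaw while setting pitch and roll to zero.
; The spin step is not scaled by DeltaSeconds, so its speed depends on frame rate.
; The construction script only calls its parent, and BeginPlay and overlap events are disabled stubs.
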(event `self.ReceiveTick`
  (params (DeltaSeconds :type "Float (single-precision)"))
  (bind _ninjastar (`self.NinjaStar`))
  (bind (_relativerotation_roll _relativerotation_pitch _relativerotation_yaw) (`KismetMathLibrary.BreakRotator` (`SceneComponent.RelativeRotation` _ninjastar)))
  (`parent.ReceiveTick` DeltaSeconds)
  (`SceneComponent.K2_SetRelativeRotation` _ninjastar (`KismetMathLibrary.MakeRotator` 0.0 0.0 (+ _relativerotation_yaw (`self.rotationIncrement`))) false false))

(fn `UserConstructionScript`
  (`parent.UserConstructionScript`))