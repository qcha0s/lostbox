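; Ninja star projectile Blueprint that damages enemy characters it overlaps.
; Each tick spins the NinjaStar component in yaw by a rotation increment and resets Damage to a fixed value.
; The Sphere component's begin-overlap event casts the other actor to Base_EnemyCharacter and passes Damage to its TakeDamage.
; The graph contains no movement or destroy-on-hit logic.
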(event `self.ReceiveTick`
  (params (DeltaSeconds :type "Float (single-precision)"))
  (bind _ninjastar (`self.NinjaStar`))
  (bind (_relativerotation_roll _relativerotation_pitch _relativerotation_yaw) (`KismetMathLibrary.BreakRotator` (`SceneComponent.RelativeRotation` _ninjastar)))
  (`parent.ReceiveTick` DeltaSeconds)
  (`SceneComponent.K2_SetRelativeRotation` _ninjastar (`KismetMathLibrary.MakeRotator` 0.0 0.0 (+ _relativerotation_yaw (`self.rotationIncrement`))) false false)
  (set `self.damage` 10.0))

(event `self.Sphere.OnComponentBeginOverlap`
  (params (OverlappedComponent :type "PrimitiveComponent Object Reference") (OtherActor :type "Actor Object Reference") (OtherComp :type "PrimitiveComponent Object Reference") (OtherBodyIndex :type Integer) (bFromSweep :type Boolean) (SweepResult :type "HitResult Structure (by ref)"))
  (bind _asbase_enemy_character (cast `/Game/Controls/Enemies/Base_EnemyCharacter` OtherActor))
  (`/Game/Controls/Base_Character.TakeDamage` _asbase_enemy_character (`self.damage`)))

(fn `UserConstructionScript`
  (`parent.UserConstructionScript`))