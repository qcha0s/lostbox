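; GreatSword_BP is a melee weapon that damages enemies its box collision begins overlapping during an attack.
; Hits count only while the owning character's DamageZone and IsAttacking flags are both set.
; An EnemiesHit list blocks repeat damage per enemy; nothing here clears it.
; The BaseDamageable_Actor damage path sits behind a constant condition, so it never runs.
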(event `self.Box.OnComponentBeginOverlap`
  (params (OverlappedComponent :type "PrimitiveComponent Object Reference") (OtherActor :type "Actor Object Reference") (OtherComp :type "PrimitiveComponent Object Reference") (OtherBodyIndex :type Integer) (bFromSweep :type Boolean) (SweepResult :type "HitResult Structure (by ref)"))
  (bind _owningcharacter (`self.OwningCharacter`))
  (`/Engine/EditorBlueprintResources/StandardMacros.IsValid` _owningcharacter
    (:`Is Valid`
      (if (and (`/Game/Controls/Players/Warrior/WarriorBaseBP.DamageZone` _owningcharacter) (`/Game/Controls/Base_Character.isAttacking` _owningcharacter))
        (bind _asbase_enemy_character (cast `/Game/Controls/Enemies/Base_EnemyCharacter` OtherActor)
          (:`then`
            (bind _hasbeenhit (`self.EnemyHasBeenHit` _asbase_enemy_character))
            (if (not _hasbeenhit)
              (`KismetArrayLibrary.Array_Add` (`self.EnemiesHit`) _asbase_enemy_character)
              (`/Game/Controls/Base_Character.TakeDamage` _asbase_enemy_character (`self.damage`))))
          (:`CastFailed`
            (bind _asbase_damageable_actor (cast `/Game/Controls/BaseDamageable_Actor` OtherActor))
            (`/Engine/EditorBlueprintResources/StandardMacros.IsValid` (`self.ActorHit`)
              (:`Is Not Valid`
                (if (not true)
                  (`/Game/Controls/BaseDamageable_Actor.TakeDamage` _asbase_damageable_actor (`self.damage`))
                  (set `self.ActorHit` _asbase_damageable_actor))))))))))

(fn `EnemyHasBeenHit`
  (params (Enemy :type "/Game/Controls/Enemies/Base_EnemyCharacter Object Reference"))
  (returns (HasBeenHit :type Boolean))
  (locals (Retval :type Boolean))
  (for _array_element (`self.EnemiesHit`)
    (if (== _array_element Enemy)
      (set `local.Retval` true)))
  (return (`local.Retval`)))

(fn `UserConstructionScript`)