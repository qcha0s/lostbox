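; Base Blueprint for the Warrior player character, which carries a greatsword and tracks whether it is attacking.
; On BeginPlay it spawns a GreatSword, sets itself as the owning character and snaps the sword to the mesh's SwordSocket.
; The BasicAttack input holds IsAttacking true while pressed and clears it on release.
; A separate Attack function only sets the same flag, with no reset of its own.
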(event `self.ReceiveBeginPlay`
  (`parent.ReceiveBeginPlay`)
  (bind _returnvalue (`|SpawnActorFromClass` "/Game/Controls/Weapons/GreatSword.GreatSword_C" (`KismetMathLibrary.MakeTransform` (0.0 0.0 0.0)) "AlwaysSpawn" "OverrideRootScale" null null))
  (set `/Game/Controls/Weapons/GreatSword.OwningCharacter` self _returnvalue)
  (`SceneComponent.K2_AttachToComponent` (`Actor.RootComponent` _returnvalue) (`self.Mesh`) "SwordSocket" "SnapToTarget" "SnapToTarget" "SnapToTarget" true))

(event `InputAction|BasicAttack`
  (params (Key :type "Key Structure"))
  (:`Pressed`
    (set `self.isAttacking` true))
  (:`Released`
    (set `self.isAttacking` false)))

(fn `Attack`
  (set `self.isAttacking` true))

(fn `UserConstructionScript`
  (`parent.UserConstructionScript`))