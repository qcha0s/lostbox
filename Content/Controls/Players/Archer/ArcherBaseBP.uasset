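; Base Blueprint for an archer player character that carries a bow and performs a basic attack.
; On BeginPlay it spawns the bow, attaches it to the mesh's BowSocket and stores normal and damaged materials.
; The BasicAttack input locks movement, calls Attack on the bow, then restores walking after a short delay, with an IsAttacking flag blocking re-entry.
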(event `self.ReceiveBeginPlay`
  (bind _returnvalue (`|SpawnActorFromClass` "/Game/Controls/Weapons/Bow.Bow_C" (`KismetMathLibrary.MakeTransform` (0.0 0.0 0.0)) "AlwaysSpawn" "OverrideRootScale" null null))
  (bind _output_get (set `self.Bow` _returnvalue))
  (`SceneComponent.K2_AttachToComponent` (`Actor.RootComponent` _output_get) (`self.Mesh`) "BowSocket" "SnapToTarget" "SnapToTarget" "SnapToTarget" true)
  (set `self.NormalMat` "/Game/Controls/Materials/Pallet_Mat.Pallet_Mat")
  (set `self.DamagedMat` "/Game/Controls/Materials/Damaged_Mat.Damaged_Mat"))

(event `InputAction|BasicAttack`
  (params (Key :type "Key Structure"))
  (:`Pressed`
    ;[0.09055 1 0] Comment
    (if (not (`self.IsAttacking`))
      (`CharacterMovementComponent.DisableMovement` (`self.CharacterMovement`))
      (`MovementComponent.StopMovementImmediately` (`self.CharacterMovement`))
      (set `self.IsAttacking` true)
      ;[1 0 0.6459] Spawn the Arrow ****Add Arrow Actor Here***
      (`/Game/Controls/Weapons/Bow.Attack` (`self.Bow`))
      (`KismetSystemLibrary.Delay` 0.2)
      (set `self.IsAttacking` false)
      (`CharacterMovementComponent.SetMovementMode` (`self.CharacterMovement`) "MOVE_Walking" 0))))

(fn `UserConstructionScript`
  (`parent.UserConstructionScript`))