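; Base Blueprint for the Archer player character, a bow-wielding ranged attacker.
; On BeginPlay it spawns a Bow_BP, snaps it to the mesh's BowSocket and sets the attack rate used by parent events.
; Attack0 only raises the IsAttacking flag.
; The separate FireWeapon event calls Shoot on the bow, passing the world rotation and scale of Arrow1.
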(event `self.ReceiveBeginPlay`
  ;[1 1 1] Attach bow, set attack rate for parent events
  (`self.MakeAndAttachBow`)
  (set `self.PlayerAttackRate` 0.8))

(event `FireWeapon`
  (bind (_returnvalue_location _returnvalue_rotation _returnvalue_scale) (`KismetMathLibrary.BreakTransform` (`SceneComponent.K2_GetComponentToWorld` (`self.Arrow1`))))
  ;[1 1 1] ShootProjectile
  (`/Game/Controls/Weapons/Bow_BP.Shoot` (`self.Bow`) _returnvalue_rotation _returnvalue_scale))

(fn `Attack_0`
  (set `self.isAttacking` true))

(fn `MakeAndAttachBow`
  (bind _returnvalue (`|SpawnActorFromClass` "/Game/Controls/Weapons/Bow_BP.Bow_BP_C" (`KismetMathLibrary.MakeTransform` (0.0 0.0 0.0)) "AlwaysSpawn" "OverrideRootScale" null null))
  (set `self.Bow` _returnvalue)
  (`SceneComponent.K2_AttachToComponent` (`Actor.RootComponent` _returnvalue) (`self.Mesh`) "BowSocket" "SnapToTarget" "SnapToTarget" "SnapToTarget" true))

(fn `UserConstructionScript`)