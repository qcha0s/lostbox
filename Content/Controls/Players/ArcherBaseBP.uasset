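; Base Blueprint for an archer player that fires a projectile and can take damage and die.
; BasicAttack stops and disables movement, spawns a FireBall at the Arrow1 transform, then restores walking after a short delay, with IsAttacking blocking re-entry.
; AffectHealth passes the delta to CalculateHealth and, if IsDead is set, destroys the actor after a delay.
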(event `/Game/TopDownBP/Blueprints/DamageInterface.Affect Health`
  (params (Delta :type "Float (single-precision)"))
  ;[1 0 0.28] Use Damage Interface Is He hurt? Set new Health. Is He dead? If he is he will animate and die.
  (`self.CalculateHealth` Delta)
  (if (`self.isDead`)
    (`KismetSystemLibrary.Delay` 4.0)
    (`self.K2_DestroyActor`)))

(event `InputAction|BasicAttack`
  (params (Key :type "Key Structure"))
  (:`Pressed`
    ;[0.09055 1 0] Comment
    (if (not (`self.IsAttacking`))
      (`CharacterMovementComponent.DisableMovement` (`self.CharacterMovement`))
      (`MovementComponent.StopMovementImmediately` (`self.CharacterMovement`))
      (set `self.IsAttacking` true)
      ;[1 0 0.6459] Spawn the Arrow ****Add Arrow Actor Here***
      (`|SpawnActorFromClass` "/Game/Controls/Weapons/FireBall.FireBall_C" (`SceneComponent.K2_GetComponentToWorld` (`self.Arrow1`)) "Undefined" "OverrideRootScale" null null)
      (`KismetSystemLibrary.Delay` 0.2)
      (set `self.IsAttacking` false)
      (`CharacterMovementComponent.SetMovementMode` (`self.CharacterMovement`) "MOVE_Walking" 0))))

(fn `UserConstructionScript`
  (`parent.UserConstructionScript`))