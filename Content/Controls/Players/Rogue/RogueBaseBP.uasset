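; RogueBaseBP is the Rogue player base Blueprint, which throws ninja stars.
; On BeginPlay it sets the attack rate, then spawns a held star actor and snaps it to a socket on the mesh.
; ThrowingStar spawns a scaled-up projectile at the held star's location with the NinjaSpawner rotation, then briefly hides the held star to fake the throw.
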(event `self.ReceiveBeginPlay`
  (`parent.ReceiveBeginPlay`)
  (set `self.PlayerAttackRate` 0.8)
  (bind _returnvalue (`|SpawnActorFromClass` "/Game/Controls/Weapons/StarInHand_BP.StarInHand_BP_C" (`KismetMathLibrary.MakeTransform` (0.0 0.0 0.0)) "AlwaysSpawn" "OverrideRootScale" null null))
  (set `self.NinjaStar` _returnvalue)
  (`SceneComponent.K2_AttachToComponent` (`Actor.RootComponent` _returnvalue) (`self.Mesh`) "NinjaStarSocket" "SnapToTarget" "SnapToTarget" "SnapToTarget" true))

(event `ThrowingStar`
  (bind _returnvalue_location (`KismetMathLibrary.BreakTransform` (`self.GetTransform` (`self.NinjaStar`))))
  (bind _ninjastar (`/Game/Controls/Weapons/StarInHand_BP.NinjaStar` (`self.NinjaStar`)))
  (`|SpawnActorFromClass` "/Game/Controls/Weapons/NinjaStarProjectile_BP.NinjaStarProjectile_BP_C" (`KismetMathLibrary.MakeTransform` _returnvalue_location (`SceneComponent.K2_GetComponentRotation` (`self.NinjaSpawner`)) (3.0 3.0 3.0)) "AlwaysSpawn" "OverrideRootScale" null null)
  (`SceneComponent.SetVisibility` _ninjastar false true)
  (`KismetSystemLibrary.Delay` 0.5)
  (`SceneComponent.SetVisibility` _ninjastar true true))

(fn `UserConstructionScript`
  (`parent.UserConstructionScript`))