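; Base Blueprint for the Rogue player character, implementing its basic ranged attack.
; On BasicAttack press, it halts movement and spawns a FireBall at the mesh's NinjaStarSocket, oriented by the NinjaSpawner component's rotation.
; An IsAttacking flag and short delay block repeat fire, after which the movement mode is set back to Walking.
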(event `InputAction|BasicAttack`
  (params (Key :type "Key Structure"))
  (bind (_returnvalue_location _returnvalue_rotation _returnvalue_scale) (`KismetMathLibrary.BreakTransform` (`SceneComponent.GetSocketTransform` (`self.Mesh`) "NinjaStarSocket" "RTS_World")))
  (:`Pressed`
    (if (not (`self.IsAttacking`))
      (`MovementComponent.StopMovementImmediately` (`self.CharacterMovement`))
      (`MovementComponent.StopMovementImmediately` (`self.CharacterMovement`))
      (`|SpawnActorFromClass` "/Game/Controls/Weapons/FireBall.FireBall_C" (`KismetMathLibrary.MakeTransform` _returnvalue_location (`SceneComponent.K2_GetComponentRotation` (`self.NinjaSpawner`)) _returnvalue_scale) "Undefined" "OverrideRootScale" null null)
      (set `self.IsAttacking` true)
      (`KismetSystemLibrary.Delay` 0.2)
      (set `self.IsAttacking` false)
      (`CharacterMovementComponent.SetMovementMode` (`self.CharacterMovement`) "MOVE_Walking" 0))))

(fn `UserConstructionScript`
  (`parent.UserConstructionScript`))