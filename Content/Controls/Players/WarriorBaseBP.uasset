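; Base player Blueprint for a warrior character, handling a basic attack, sword damage and death.
; The BasicAttack input briefly raises IsAttacking, then restores walking movement, though the branch that halts movement is unconnected.
; Sphere overlaps with DamageInterface actors carrying a different first tag call AffectHealth with SwordDamage.
; AffectHealth runs CalculateHealth and, on death, disables input and destroys the actor after a delay.
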(event `InputAction|BasicAttack`
  (params (Key :type "Key Structure"))
  (:`Pressed`
    ;[1 1 1] Attacking
    (set `self.IsAttacking` true)
    (`KismetSystemLibrary.Delay` 0.3)
    (set `self.IsAttacking` false)
    (`CharacterMovementComponent.SetMovementMode` (`self.CharacterMovement`) "MOVE_Walking" 0)))

(event `/Game/TopDownBP/Blueprints/DamageInterface.Affect Health`
  (params (Delta :type "Float (single-precision)"))
  ;[1 1 1] Health calculations and handling death
  (`self.CalculateHealth` Delta)
  (if (`self.isDead`)
    (`self.DisableInput` null)
    (`KismetSystemLibrary.Delay` 4.0)
    (`self.K2_DestroyActor`)))

(event `self.Sphere.OnComponentBeginOverlap`
  (params (OverlappedComponent :type "PrimitiveComponent Object Reference") (OtherActor :type "Actor Object Reference") (OtherComp :type "PrimitiveComponent Object Reference") (OtherBodyIndex :type Integer) (bFromSweep :type Boolean) (SweepResult :type "HitResult Structure (by ref)"))
  (if (`KismetSystemLibrary.DoesImplementInterface` OtherActor "/Game/TopDownBP/Blueprints/DamageInterface.DamageInterface_C")
    (if (not (== (`|GetArrayItem` (`self.Tags`)) (`|GetArrayItem` (`Actor.Tags` OtherActor))))
      (`/Game/TopDownBP/Blueprints/DamageInterface.Affect Health` (`self.SwordDamage`)))))

(fn `UserConstructionScript`
  (`parent.UserConstructionScript`))