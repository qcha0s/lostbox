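; WizardBaseBP is the base wizard player character, which carries a staff and shoots fireballs.
; On BeginPlay it runs parent logic, spawns a Staff owned by itself, snaps it to the mesh's StaffSocket and sets the attack rate used by parent events.
; ShootFireBall spawns a FireBall at the staff's arrow location, taking rotation and scale from the character's SpellSpawn component.
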(event `self.ReceiveBeginPlay`
  ;[1 1 1] Attach Staff, get reference to it and set attack rate for parent events
  (`parent.ReceiveBeginPlay`)
  (bind _returnvalue (`|SpawnActorFromClass` "/Game/Controls/Weapons/Staff.Staff_C" (`KismetMathLibrary.MakeTransform` (0.0 0.0 0.0)) "AlwaysSpawn" "OverrideRootScale" null null))
  (set `/Game/Controls/Weapons/Staff.OwningCharacter` self _returnvalue)
  (set `self.Staff` _returnvalue)
  (`SceneComponent.K2_AttachToComponent` (`Actor.RootComponent` _returnvalue) (`self.Mesh`) "StaffSocket" "SnapToTarget" "SnapToTarget" "SnapToTarget" true)
  (set `self.PlayerAttackRate` 0.6))

(event `ShootFireBall`
  (bind (_returnvalue_location _returnvalue_rotation _returnvalue_scale) (`KismetMathLibrary.BreakTransform` (`SceneComponent.K2_GetComponentToWorld` (`self.SpellSpawn`))))
  ;[1 1 1] ShootProjectile
  (`|SpawnActorFromClass` "/Game/Controls/Weapons/FireBall.FireBall_C" (`KismetMathLibrary.MakeTransform` (`SceneComponent.K2_GetComponentLocation` (`/Game/Controls/Weapons/Staff.Arrow` (`self.Staff`))) _returnvalue_rotation _returnvalue_scale) "AlwaysSpawn" "OverrideRootScale" null null))

(fn `UserConstructionScript`
  (`parent.UserConstructionScript`))