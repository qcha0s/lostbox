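; Base Blueprint for the Wizard player character, handling its staff, fireball attack and death.
; On BeginPlay it spawns a staff, sets itself as owner and snaps it to the mesh's StaffSocket.
; BasicAttack input freezes movement and flags casting, or restores walking if already casting, while ShootFireBall spawns the projectile at the staff's arrow with SpellSpawn's rotation.
; Death disables input and movement, plays a sound, then respawns after a delay.
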(event `/Game/Controls/Base_Character.Death`
  (bind _charactermovement (`self.CharacterMovement`))
  (`self.DisableInput` (`GameplayStatics.GetPlayerController` 0))
  (`CharacterMovementComponent.DisableMovement` _charactermovement)
  (`MovementComponent.StopMovementImmediately` _charactermovement)
  (`GameplayStatics.PlaySoundAtLocation` null (`self.K2_GetActorLocation`))
  (`KismetSystemLibrary.Delay` 4.0)
  (`self.Respawn`))

(event `self.ReceiveBeginPlay`
  (`parent.ReceiveBeginPlay`)
  (bind _returnvalue (`|SpawnActorFromClass` "/Game/Controls/Weapons/Staff.Staff_C" (`KismetMathLibrary.MakeTransform` (0.0 0.0 0.0)) "AlwaysSpawn" "OverrideRootScale" null null))
  (set `/Game/Controls/Weapons/Staff.OwningCharacter` self _returnvalue)
  (set `self.Staff` _returnvalue)
  (`SceneComponent.K2_AttachToComponent` (`Actor.RootComponent` _returnvalue) (`self.Mesh`) "StaffSocket" "SnapToTarget" "SnapToTarget" "SnapToTarget" true))

(event `InputAction|BasicAttack`
  (params (Key :type "Key Structure"))
  (bind _charactermovement (`self.CharacterMovement`))
  ;[1 1 1] Attack Anim Handling
  (:`Pressed`
    (if (`self.IsCastingSpell`)
      (`CharacterMovementComponent.SetMovementMode` _charactermovement "MOVE_Walking" 0)
      (else
        (`CharacterMovementComponent.DisableMovement` _charactermovement)
        (`MovementComponent.StopMovementImmediately` _charactermovement)
        (set `self.IsCastingSpell` true)))))

(event `ShootFireBall`
  (bind (_returnvalue_location _returnvalue_rotation _returnvalue_scale) (`KismetMathLibrary.BreakTransform` (`SceneComponent.K2_GetComponentToWorld` (`self.SpellSpawn`))))
  (`|SpawnActorFromClass` "/Game/Controls/Weapons/FireBall.FireBall_C" (`KismetMathLibrary.MakeTransform` (`SceneComponent.K2_GetComponentLocation` (`/Game/Controls/Weapons/Staff.Arrow` (`self.Staff`))) _returnvalue_rotation _returnvalue_scale) "AlwaysSpawn" "OverrideRootScale" null null))

(fn `UserConstructionScript`
  (`parent.UserConstructionScript`))