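; Base Blueprint for a ranged Wizard player character that casts fireballs and handles its own death.
; The BasicAttack input, gated by IsCastingSpell, halts movement, flags IsAttacking and spawns a FireBall at the SpellSpawn transform.
; A short delay then clears the attack flag and restores walking.
; The Death event plays a sound at the actor's location and destroys it after a delay.
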(event `self.Death`
  (`GameplayStatics.PlaySoundAtLocation` null (`self.K2_GetActorLocation`))
  (`KismetSystemLibrary.Delay` 4.0)
  (`self.K2_DestroyActor`))

(event `InputAction|BasicAttack`
  (params (Key :type "Key Structure"))
  (bind _charactermovement (`self.CharacterMovement`))
  ;[1 1 1] Attack Anim Handling
  (:`Pressed`
    (if (`self.IsCastingSpell`)
      (`CharacterMovementComponent.DisableMovement` _charactermovement)
      (`MovementComponent.StopMovementImmediately` _charactermovement)
      (set `self.isAttacking` true)
      (`|SpawnActorFromClass` "/Game/Controls/Weapons/FireBall.FireBall_C" (`SceneComponent.K2_GetComponentToWorld` (`self.SpellSpawn`)) "Undefined" "OverrideRootScale" null null)
      (`KismetSystemLibrary.Delay` 0.3)
      (set `self.isAttacking` false)
      (`CharacterMovementComponent.SetMovementMode` (`self.CharacterMovement`) "MOVE_Walking" 0))))

(fn `UserConstructionScript`
  (`parent.UserConstructionScript`))