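; Base Blueprint for a mummy enemy that attacks the player character when it enters a sphere trigger.
; Overlap stores the player reference and starts a looping Attack timer that sets IsAttacking; leaving clears both.
; A separate AttackPlayer event applies the mummy's damage to the stored player.
; A Death event plays the death animation on the mesh.
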(event `self.Sphere.OnComponentBeginOverlap`
  (params (OverlappedComponent :type "PrimitiveComponent Object Reference") (OtherActor :type "Actor Object Reference") (OtherComp :type "PrimitiveComponent Object Reference") (OtherBodyIndex :type Integer) (bFromSweep :type Boolean) (SweepResult :type "HitResult Structure (by ref)"))
  ;[1 1 1] Cause Damage to player
  (`/Engine/EditorBlueprintResources/StandardMacros.IsValid` (`self.PlayerRef`)
    (:`Is Not Valid`
      (bind _asbase_player_character (cast `/Game/Controls/Players/Base_PlayerCharacter` OtherActor))
      (set `self.PlayerRef` _asbase_player_character)
      (`self.Attack`)
      (`KismetSystemLibrary.K2_SetTimer` null "Attack" (`self.AttackRate`) true))))

(event `self.Sphere.OnComponentEndOverlap`
  (params (OverlappedComponent :type "PrimitiveComponent Object Reference") (OtherActor :type "Actor Object Reference") (OtherComp :type "PrimitiveComponent Object Reference") (OtherBodyIndex :type Integer))
  ;[1 1 1] Cause Damage to player
  (`/Engine/EditorBlueprintResources/StandardMacros.IsValid` (`self.PlayerRef`)
    (:`Is Valid`
      (bind _asbase_player_character (cast `/Game/Controls/Players/Base_PlayerCharacter` OtherActor))
      (if (== (`self.PlayerRef`) _asbase_player_character)
        (set `self.PlayerRef` null)
        (`KismetSystemLibrary.K2_ClearTimer` null "Attack")
        (set `self.isAttacking` false)))))

(event `AttackPlayer`
  (bind _playerref (`self.PlayerRef`))
  (`/Engine/EditorBlueprintResources/StandardMacros.IsValid` _playerref
    (:`Is Valid`
      (`self.TakeDamage` _playerref (`self.MummyDamage`)))))

(event `self.Death`
  (`SkeletalMeshComponent.PlayAnimation` (`self.Mesh`) "/Game/TopDownBP/Characters/Mummy/Mummy_Death_Anim.Mummy_Death_Anim" false))

(fn `Attack`
  (set `self.isAttacking` true))

(fn `UserConstructionScript`
  (`parent.UserConstructionScript`))