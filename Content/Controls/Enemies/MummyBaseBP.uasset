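; MummyBaseBP is the base mummy enemy Blueprint, handling health, death and attack damage to the player.
; AffectHealth runs CalculateHealth and, once IsDead is set, destroys the actor after a short delay.
; While IsAttacking is set, DamageVolume overlaps with DamageInterface actors whose first tag differs trigger AffectHealth with AttackDamage, then clear the attack flag.
; Unconnected movement-stopping nodes remain as a possible fix for sliding during attacks.
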(event `self.Affect Health`
  (params (Delta :type "Float (single-precision)"))
  ;[1 1 1] Calculate health and handle death
  (`self.CalculateHealth` Delta)
  (if (`self.isDead`)
    (`KismetSystemLibrary.Delay` 4.0)
    (`self.K2_DestroyActor`)))

(event `self.DamageVolume.OnComponentBeginOverlap`
  (params (OverlappedComponent :type "PrimitiveComponent Object Reference") (OtherActor :type "Actor Object Reference") (OtherComp :type "PrimitiveComponent Object Reference") (OtherBodyIndex :type Integer) (bFromSweep :type Boolean) (SweepResult :type "HitResult Structure (by ref)"))
  ;[1 1 1] Cause Damage to player
  (if (`self.IsAttacking`)
    (if (`KismetSystemLibrary.DoesImplementInterface` OtherActor "/Game/TopDownBP/Blueprints/DamageInterface.DamageInterface_C")
      (if (not (== (`|GetArrayItem` (`self.Tags`)) (`|GetArrayItem` (`Actor.Tags` OtherActor))))
        (set `self.IsAttacking` true)
        (`self.Affect Health` (`self.AttackDamage`))
        (set `self.IsAttacking` false)))))

(fn `UserConstructionScript`
  (`parent.UserConstructionScript`))