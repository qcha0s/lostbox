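; Dragon enemy character that periodically halts to roar or breathe fire, with its scale, material and health set on BeginPlay.
; Looping timers set the roar or fire-breath state flags and stop movement, with roars random and skipped while firing.
; StartFire and StopFire toggle a rapid fireball-spawning timer, while RoarFireBall spawns a larger fire attack, both from the mesh's ArrowSocket.
; These functions, StartMove and the flag resets are driven from outside this graph.
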(event `self.ReceiveTick`
  (params (DeltaSeconds :type "Float (single-precision)")))

(event `self.ReceiveBeginPlay`
  (`self.SetActorScale3D` (2.0 2.0 2.0))
  (set `self.NormalMat` "/Game/Controls/Materials/Pallet_Mat.Pallet_Mat")
  (`KismetSystemLibrary.K2_SetTimer` null "DragonRoar" 6.0 true)
  (`KismetSystemLibrary.K2_SetTimer` null "FireBreath" 8.0 true)
  (bind _output_get (set `self.MaxHealth` 200.0))
  (set `self.CurrentHealth` _output_get))

(event `StopMove`
  (`MovementComponent.StopMovementImmediately` (`self.CharacterMovement`))
  (set `CharacterMovementComponent.MaxWalkSpeed` 0.0 (`self.CharacterMovement`)))

(event `StartMove`
  (set `CharacterMovementComponent.MaxWalkSpeed` 200.0 (`self.CharacterMovement`)))

(fn `DragonRoar`
  (if (`KismetMathLibrary.RandomBoolWithWeight` 0.5)
    (if (not (`self.IsFiringFireBalls`))
      (set `self.IsRoaring` true)
      (`self.StopMove`))))

(fn `FireBreath`
  (set `self.IsFiringFireBalls` true)
  (`self.StopMove`))

(fn `RoarFireBall`
  (bind _returnvalue (`SceneComponent.GetSocketTransform` (`self.Mesh`) "ArrowSocket" "RTS_World"))
  (`|SpawnActorFromClass` "/Game/Controls/Weapons/DragonProjectile/DragonFireAttack.DragonFireAttack_C" (`KismetMathLibrary.MakeTransform` (.location _returnvalue) (`SceneComponent.K2_GetComponentRotation` (`self.FireShot_1`)) (3.0 3.0 3.0)) "AlwaysSpawn" "OverrideRootScale" null null)
  (`GameplayStatics.PlaySoundAtLocation` "/Game/SFX/Characters/Enemies/Dragon/BreathFire/DragonFire.DragonFire" (.location _returnvalue)))

(fn `SpawnFireBall`
  (bind _returnvalue (`SceneComponent.GetSocketTransform` (`self.Mesh`) "ArrowSocket" "RTS_World"))
  (`|SpawnActorFromClass` "/Game/Controls/Weapons/DragonProjectile/DragonFireBall.DragonFireBall_C" (`KismetMathLibrary.MakeTransform` (.location _returnvalue) (`KismetMathLibrary.MakeRotator` 0.0 0.0 (.yaw (.rotation _returnvalue)))) "AlwaysSpawn" "OverrideRootScale" null null)
  (`GameplayStatics.PlaySoundAtLocation` "/Game/SFX/Characters/Enemies/Dragon/BreathFire/DragonFire.DragonFire" (.location _returnvalue)))

(fn `StartFire`
  (`KismetSystemLibrary.K2_SetTimer` null "SpawnFireBall" 0.1 true))

(fn `StopFire`
  (`KismetSystemLibrary.K2_ClearTimer` null "SpawnFireBall"))

(fn `UserConstructionScript`)