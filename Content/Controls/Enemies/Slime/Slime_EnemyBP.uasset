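; Slime enemy that damages the player on capsule hit and splits into two smaller slimes when it dies.
; Looping Shrink and Grow timers hand off to each other, trading height against width for a squash-and-stretch wobble.
; An IsAttacking flag, cleared on a later hit after an attack-rate delay, gates damage.
; Death spawns two half-scale copies (the second then zero-scaled) with set health and HasSplit, so they cannot split again.
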(event `self.ReceiveBeginPlay`
  (bind _returnvalue (`self.GetActorScale3D`))
  (set `self.OriginalScale` _returnvalue)
  (set `self.DecrementValue` (/ (.z _returnvalue) 40.0))
  (`KismetSystemLibrary.K2_SetTimer` null "Shrink" 0.1 true)
  (set `self.NormalMat` "/Game/Controls/Enemies/Slime/SlimeMaterial.SlimeMaterial")
  (set `self.DamagedMat` "/Game/Controls/Enemies/Slime/SlimeDamagedMat.SlimeDamagedMat"))

(event `self.CapsuleComponent.OnComponentHit`
  (params (HitComponent :type "PrimitiveComponent Object Reference") (OtherActor :type "Actor Object Reference") (OtherComp :type "PrimitiveComponent Object Reference") (NormalImpulse :type "Vector Structure") (Hit :type "HitResult Structure (by ref)"))
  ;[1 1 1] Slime and Enemy Take Damage
  (if (`self.isAttacking`)
    (`KismetSystemLibrary.Delay` (`self.AttackRate`))
    (set `self.isAttacking` false)
    (else
      (set `self.isAttacking` true)
      (bind _asbase_player_character (cast `/Game/Controls/Players/Base_PlayerCharacter` OtherActor))
      (`self.TakeDamage` _asbase_player_character (`self.SlimeDamage`)))))

(event `self.Death`
  ;[1 1 1] Slime Death
  (`self.CheckSplit`))

(fn `CheckSplit`
  ;[1 1 1] Split The Slime
  (if (`self.HasSplit`)
    (`self.K2_DestroyActor`)
    (else
      (`self.SpawnSplitSlimes`))))

(fn `Grow`
  (bind (_returnvalue_x _returnvalue_y _returnvalue_z) (`KismetMathLibrary.BreakVector` (`self.GetActorScale3D`)))
  (bind (_returnvalue_x_2 _returnvalue_y_2 _returnvalue_z_2) (`KismetMathLibrary.BreakVector` (`self.GetActorScale3D`)))
  (bind _decrementvalue (`self.DecrementValue`))
  (bind (_originalscale_x _originalscale_y _originalscale_z) (`KismetMathLibrary.BreakVector` (`self.OriginalScale`)))
  (`self.SetActorScale3D` (`KismetMathLibrary.MakeVector` (- _returnvalue_x_2 _decrementvalue) (- _returnvalue_y_2 _decrementvalue) (+ _returnvalue_z_2 _decrementvalue)))
  (if (>= _returnvalue_z _originalscale_z)
    (`KismetSystemLibrary.K2_SetTimer` null "Shrink" 0.05 true)
    (`KismetSystemLibrary.K2_ClearTimer` null "Grow")))

(fn `Shrink`
  (bind (_returnvalue_x _returnvalue_y _returnvalue_z) (`KismetMathLibrary.BreakVector` (`self.GetActorScale3D`)))
  (bind (_returnvalue_x_2 _returnvalue_y_2 _returnvalue_z_2) (`KismetMathLibrary.BreakVector` (`self.GetActorScale3D`)))
  (bind _decrementvalue (`self.DecrementValue`))
  (bind (_originalscale_x _originalscale_y _originalscale_z) (`KismetMathLibrary.BreakVector` (`self.OriginalScale`)))
  (`self.SetActorScale3D` (`KismetMathLibrary.MakeVector` (+ _returnvalue_x_2 _decrementvalue) (+ _returnvalue_y_2 _decrementvalue) (- _returnvalue_z_2 _decrementvalue)))
  (if (<= _returnvalue_z (/ _originalscale_z 1.5))
    (`KismetSystemLibrary.K2_SetTimer` null "Grow" 0.05 true)
    (`KismetSystemLibrary.K2_ClearTimer` null "Shrink")))

(fn `SpawnSplitSlimes`
  (bind _returnvalue (`KismetMathLibrary.MakeTransform` (.location (`self.GetTransform`)) (.rotation (`self.GetTransform`)) (/ (`self.OriginalScale`) 2.0)))
  (bind _returnvalue_2 (`|SpawnActorFromClass` "Slime_EnemyBP_C" _returnvalue "Undefined" "OverrideRootScale" null null))
  (set `/Game/Controls/Enemies/Slime/Slime_EnemyBP.HasSplit` true _returnvalue_2)
  (set `/Game/Controls/Base_Character.Health` 50.0 _returnvalue_2)
  (bind _returnvalue_3 (`|SpawnActorFromClass` "Slime_EnemyBP_C" _returnvalue "Undefined" "OverrideRootScale" null null))
  (`self.SetActorScale3D` _returnvalue_3 (0.0 0.0 0.0))
  (set `/Game/Controls/Enemies/Slime/Slime_EnemyBP.HasSplit` true _returnvalue_3)
  (set `/Game/Controls/Base_Character.Health` 50.0 _returnvalue_3)
  (`self.K2_DestroyActor`))

(fn `UserConstructionScript`)